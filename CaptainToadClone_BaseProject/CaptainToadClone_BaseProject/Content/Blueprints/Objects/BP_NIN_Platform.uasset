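; Platform actor that moves between two points when its CallAction event is switched on or off.
; At BeginPlay it converts PointA and PointB from relative offsets to world positions.
; CallAction targets PointB when active and PointA otherwise, then restarts a shared timeline.
; Each update lerps from the current location, not a fixed start, so motion is non-linear, and moves without sweep.
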(event EventBeginPlay
  (bind _returnvalue (Transformation|GetActorLocation))
  (Variables|Default|SetPointA (+ _returnvalue (Variables|Default|GetPointA)))
  (Variables|Default|SetPointB (+ _returnvalue (Variables|Default|GetPointB))))

(event EventCallAction
  (params (active :type Boolean))
  (if active
    (Variables|Default|SetcurrentPoint (Variables|Default|GetPointB))
    (bind _time (Timeline|Timeline PlayFromStart)
      (:Update
        (Transformation|SetActorLocation (Math|Vector|Lerp(Vector) (Transformation|GetActorLocation) (Variables|Default|GetcurrentPoint) _time) false false)))
    (else
      (Variables|Default|SetcurrentPoint (Variables|Default|GetPointA))
      (Timeline|Timeline PlayFromStart))))

(fn ConstructionScript
  (|CallParentFunction))