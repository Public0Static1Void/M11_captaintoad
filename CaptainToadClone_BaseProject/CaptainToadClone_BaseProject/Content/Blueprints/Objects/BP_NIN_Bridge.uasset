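; BP_NIN_Bridge is a bridge actor that rotates 90 degrees in yaw when triggered through CallAction.
; Tick advances a lerp alpha and calls LerpRotation to blend between stored start and target rotations.
; Non-additive mode swings back on deactivation, while Additive mode holds position and re-bases the target for another quarter turn.
; Deactivation is ignored while a turn is still in progress.
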(event EventBeginPlay
  (bind _output_get (Variables|Default|SetstartRot (Transformation|GetActorRotation)))
  (Variables|Default|SetauxRot _output_get)
  (Variables|Default|SettargetRot (Math|Rotator|MakeRotator (.roll (Variables|Default|GetstartRot)) (.pitch (Variables|Default|GetstartRot)) (+ (.yaw (Variables|Default|GetstartRot)) 9e+01))))

(event EventTick
  (params (DeltaSeconds :type Float%20%28single-precision%29))
  ;[0.15 0.15 0.15 0.5] Rotation
  (Variables|Default|SetlerpAmount (+ (* DeltaSeconds (Variables|Default|GetlerpSum)) (Variables|Default|GetlerpAmount)))
  (if (< (Variables|Default|GetlerpAmount) 1.0)
    (CallFunction|LerpRotation (Variables|Default|GetlerpAmount) (Variables|Default|GetstartRot) (Variables|Default|GettargetRot))))

(event EventCallAction
  (params (active :type Boolean))
  (bind _returnvalue (Transformation|GetActorRotation))
  (if active
    (if (Variables|Default|Getadditive)
      _
      (else
        (Variables|Default|SetstartRot (Transformation|GetActorRotation))
        (Variables|Default|SettargetRot (Math|Rotator|MakeRotator (.roll (Variables|Default|GetstartRot)) (.pitch (Variables|Default|GetstartRot)) (+ (.yaw (Variables|Default|GetstartRot)) 9e+01)))))
    (Variables|Default|SetlerpSum 1.0)
    (Variables|Default|SetlerpAmount 0.0)
    (elif (not (< (Variables|Default|GetlerpAmount) 1.0))
      (if (Variables|Default|Getadditive)
        ;[0.15 0.15 0.15 0.5] Additive off
        (Variables|Default|SetstartRot (Transformation|GetActorRotation))
        (Variables|Default|SettargetRot (Math|Rotator|MakeRotator (.roll (Variables|Default|GetstartRot)) (.pitch (Variables|Default|GetstartRot)) (+ (.yaw (Variables|Default|GetstartRot)) 9e+01)))
        (Variables|Default|SetlerpAmount 0.0)
        (Variables|Default|SetlerpSum 0.0)
        (else
          ;[0.15 0.15 0.15 0.5] Non-Additive off
          (Variables|Default|SettargetRot (Math|Rotator|MakeRotator (.roll _returnvalue) (.pitch _returnvalue) (- (.yaw _returnvalue) 9e+01)))
          (Variables|Default|SetstartRot (Transformation|GetActorRotation))
          (Variables|Default|SetlerpSum 1.0)
          (Variables|Default|SetlerpAmount 0.0))))))

(fn ConstructionScript
  (|CallParentFunction))

(fn LerpRotation
  (params (Time :type Float%20%28double-precision%29) (StartRot :type Rotator) (TargetRot :type Rotator))
  (Transformation|SetActorRotation (Math|Rotator|Lerp(Rotator) StartRot TargetRot Time)))