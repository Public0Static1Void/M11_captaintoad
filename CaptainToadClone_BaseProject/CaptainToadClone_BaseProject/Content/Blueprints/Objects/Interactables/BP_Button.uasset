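; Weighted button that switches linked actors on or off when an object enters or leaves its trigger box.
; CheckMass forces physics on for the overlapping actor's static mesh and compares its mass to ActivationMass.
; A heavy enough object sends CallActionMessage to every AddedActors entry and snaps to SnapPoint with physics disabled.
; On exit, a qualifying object sends the off message, regains physics and detaches.
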(event OnComponentBeginOverlap(Box)
  (params (OverlappedComponent :type Primitive%20Component%20Object%20Reference) (OtherActor :type Actor%20Object%20Reference) (OtherComp :type Primitive%20Component%20Object%20Reference) (OtherBodyIndex :type Integer) (bFromSweep :type Boolean) (SweepResult :type Hit%20Result%20Structure%20%28by%20ref%29))
  (bind _returnvalue (Actor|GetComponentbyClass OtherActor "/Script/Engine.StaticMeshComponent"))
  ;[0.15 0.15 0.15 0.5] Enter collision
  (bind _valid (CallFunction|CheckMass OtherActor))
  (if _valid
    (for _array_element (Variables|Default|Getadded_actors)
      (Class|BISignalReciever|CallAction(Message) _array_element true)
      ;;[0.15 0.15 0.15 0.5] Set the actor at the top of the button
      (Physics|SetSimulatePhysics _returnvalue false)
      (Transformation|AttachComponentToComponent _returnvalue (Variables|Default|GetSnapPoint) "None" "SnapToTarget" "SnapToTarget" "KeepWorld" true))))

(event OnComponentEndOverlap(Box)
  (params (OverlappedComponent :type Primitive%20Component%20Object%20Reference) (OtherActor :type Actor%20Object%20Reference) (OtherComp :type Primitive%20Component%20Object%20Reference) (OtherBodyIndex :type Integer))
  (bind _returnvalue (Actor|GetComponentbyClass OtherActor "/Script/Engine.StaticMeshComponent"))
  ;[0.15 0.15 0.15 0.5] Exit collision
  (bind _valid (CallFunction|CheckMass OtherActor))
  (Physics|SetSimulatePhysics _returnvalue false)
  (if _valid
    (for _array_element (Variables|Default|Getadded_actors)
      (Class|BISignalReciever|CallAction(Message) _array_element false))
    (Physics|SetSimulatePhysics _returnvalue true)
    (Transformation|DetachFromComponent _returnvalue "KeepWorld" "KeepWorld" "KeepRelative" false)))

(event EventBeginPlay)

(fn ConstructionScript)

(fn CheckMass
  (params (Comp :type Actor%20Object%20Reference))
  (bind _returnvalue (Actor|GetComponentbyClass Comp "/Script/Engine.StaticMeshComponent"))
  (Utilities|IsValid _returnvalue
    (:Is%20Valid
      (Physics|SetSimulatePhysics _returnvalue true)
      (if (Physics|IsSimulatingPhysics _returnvalue "None")
        (return (>= (Physics|GetMass _returnvalue) (Variables|Default|GetactivationMass)))))))