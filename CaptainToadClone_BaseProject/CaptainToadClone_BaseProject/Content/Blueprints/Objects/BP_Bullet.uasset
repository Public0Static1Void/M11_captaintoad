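; BP_Bullet is a bullet actor that damages players and enemies and destroys itself after five seconds or on overlap.
; When its static mesh overlaps an actor tagged Player or Enemy, it applies damage.
; Any other overlap runs a sphere query for nearby Pawn-type objects and pushes those with physics-simulating static meshes radially away using a velocity-change impulse.
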(event OnComponentBeginOverlap(StaticMesh)
  (params (OverlappedComponent :type Primitive%20Component%20Object%20Reference) (OtherActor :type Actor%20Object%20Reference) (OtherComp :type Primitive%20Component%20Object%20Reference) (OtherBodyIndex :type Integer) (bFromSweep :type Boolean) (SweepResult :type Hit%20Result%20Structure%20%28by%20ref%29))
  (if (or (Actor|ActorHasTag OtherActor "Player") (Actor|ActorHasTag OtherActor "Enemy"))
    ;[0.15 0.15 0.15 0.5] Damage to player/enemy
    (Game|Damage|ApplyDamage OtherActor 1.0 0 self)
    (else
      (bind _outactors (Collision|SphereOverlapActors (Transformation|GetActorLocation) 2e+02 (Utilities|Array|MakeArray "ObjectTypeQuery3") 0 (Utilities|Array|MakeArray self)))
      (for _array_element _outactors
        (Utilities|IsValid _array_element
          (:Is%20Valid
            (Utilities|IsValid (Actor|GetComponentbyClass _array_element "/Script/Engine.StaticMeshComponent")
              (:Is%20Valid
                (if (Physics|IsSimulatingPhysics (Actor|GetComponentbyClass _array_element "/Script/Engine.StaticMeshComponent") "None")
                  (Physics|AddImpulse (Actor|GetComponentbyClass _array_element "/Script/Engine.StaticMeshComponent") (* (Math|Vector|Normalize (- (Transformation|GetActorLocation _array_element) (Transformation|GetActorLocation))) 5e+02) "None" true)))))))))
  (Actor|DestroyActor))

(event EventBeginPlay
  (Utilities|FlowControl|Delay 5.0)
  (Actor|DestroyActor))

(fn ConstructionScript)