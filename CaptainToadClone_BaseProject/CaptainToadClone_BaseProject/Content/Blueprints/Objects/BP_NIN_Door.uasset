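; BP_NIN_Door is a door actor that rotates its pivot when CallAction fires.
; CallAction captures the actor's rotation and replays a timeline from the start, which lerps the pivot's world rotation toward that rotation with yaw zeroed.
; The active flag sets a yaw offset, but its addition to the starting yaw is unconnected, so both states share the same target.
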(event EventCallAction
  (params (active :type Boolean))
  (Variables|Default|SetstartRot (Transformation|GetActorRotation))
  (if active
    (Variables|Default|Setrot 9e+01)
    (bind _time (Timeline|RotTimeline PlayFromStart)
      (:Update
        (Transformation|SetWorldRotation (Variables|Default|GetPivot) (Math|Rotator|Lerp(Rotator) (Variables|Default|GetstartRot) (Math|Rotator|MakeRotator (.roll (Variables|Default|GetstartRot)) (.pitch (Variables|Default|GetstartRot)) 0.0) _time) false false)))
    (else
      (Variables|Default|Setrot 0.0)
      (Timeline|RotTimeline PlayFromStart))))

(fn ConstructionScript
  (|CallParentFunction))