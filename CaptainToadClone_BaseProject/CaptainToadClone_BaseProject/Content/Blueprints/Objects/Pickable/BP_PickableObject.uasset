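; BP_PickableObject is an object that can be picked up and tossed, driven by Attach and Detach events.
; Attach disables physics on its static mesh and snaps it to the supplied grab component.
; Detach releases the passed actor's root component in world space, re-enables mesh physics and applies a mass-independent impulse along that actor's forward and up vectors.
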(event Custom|Attach
  (params (attached_actor :type Actor%20Object%20Reference) (grab_component :type Scene%20Component%20Object%20Reference))
  (bind _self self)
  (bind _returnvalue (Actor|GetComponentbyClass _self "/Script/Engine.StaticMeshComponent"))
  (Physics|SetSimulatePhysics _returnvalue false)
  (bind _returnvalue_2 (Transformation|AttachComponentToComponent _returnvalue grab_component "None" "SnapToTarget" "SnapToTarget" "KeepRelative" false))
  (if _returnvalue_2
    _))

(event Custom|Detach
  (params (attached_actor :type Actor%20Object%20Reference))
  (bind _self self)
  (bind _returnvalue (Actor|GetComponentbyClass _self "/Script/Engine.StaticMeshComponent"))
  (Transformation|DetachFromComponent (Variables|/Script/Engine.Actor|GetRootComponent attached_actor) "KeepWorld" "KeepWorld" "KeepRelative" false)
  (Physics|SetSimulatePhysics _returnvalue true)
  (Physics|AddImpulse _returnvalue (* (+ (Transformation|GetActorForwardVector attached_actor) (Transformation|GetActorUpVector attached_actor)) 150) "None" true))

(fn ConstructionScript)