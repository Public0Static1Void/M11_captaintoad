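; AC_HealthSystem is an actor component that tracks health for a Character owner, starting at MaxHealth on BeginPlay.
; Bound add and remove events change Health: healing clamps to MaxHealth, while damage prints the value, launches the character along the knock direction and calls Die at zero or below.
; A dynamic-material hit flash, tinting BaseColor red for a second, is present but disconnected.
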(event Custom|AddHealth_Event
  (params (amount :type Float%20%28double-precision%29))
  (bind _maxhealth (Variables|Default|GetMaxHealth))
  (bind _output_get (Variables|Default|SetHealth (+ amount (Variables|Default|GetHealth))))
  (if (> _output_get _maxhealth)
    (Variables|Default|SetHealth _maxhealth)))

(event Custom|RemoveHealth_Event
  (params (amount :type Float%20%28double-precision%29) (knockDirection :type Vector))
  (bind _output_get (Variables|Default|SetHealth (- (Variables|Default|GetHealth) amount)))
  (Development|PrintString (Utilities|String|ToString(Float) _output_get))
  (Character|LaunchCharacter (Variables|Default|Getbp_char) knockDirection false false)
  (if (<= _output_get 0.0)
    (Default|CallDie)))

(event EventBeginPlay
  (EventDispatchers|BindEventtoAddHealth (delegate Custom|AddHealth_Event))
  (EventDispatchers|BindEventtoRemoveHealth (delegate Custom|RemoveHealth_Event))
  (Variables|Default|SetHealth (Variables|Default|GetMaxHealth))
  (bind _ascharacter (Utilities|Casting|CastToCharacter (Components|GetOwner)))
  (Variables|Default|Setbp_char _ascharacter))

(fn ChangeMaterialColors
  (params (materials :type Material%20Instance%20Dynamic%20Object%20Reference) (color :type Linear%20Color%20Structure))
  (Rendering|Material|SetVectorParameterValue materials "BaseColor" color :!class /Script/Engine.MaterialInstanceDynamic))