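; BP_enemy is an enemy that deals contact damage to BP_Character and can itself be damaged and killed.
; Capsule hits apply damage, gated by a CanDamage flag that re-arms after a short delay.
; The flag clears before the character cast, so hitting any other actor leaves it disabled.
; Incoming damage is forwarded to the health system component, whose Die event destroys the enemy.
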(event OnComponentHit(Capsule)
  (params (HitComponent :type Primitive%20Component%20Object%20Reference) (OtherActor :type Actor%20Object%20Reference) (OtherComp :type Primitive%20Component%20Object%20Reference) (NormalImpulse :type Vector :default "0, 0, 0") (Hit :type Hit%20Result%20Structure%20%28by%20ref%29))
  (if (Variables|Default|GetcanDamage)
    (Variables|Default|SetcanDamage false)
    (Utilities|Casting|CastToBP_Character OtherActor)
    (Game|Damage|ApplyDamage OtherActor 1.0 0 0)
    (Utilities|FlowControl|Delay 0.75)
    (Variables|Default|SetcanDamage true)))

(event Die(AC_HealthSystem)
  (Actor|DestroyActor))

(event EventBeginPlay)

(event EventTick
  (params (DeltaSeconds :type Float%20%28single-precision%29)))

(event Game|Damage|EventAnyDamage
  (params (Damage :type Float%20%28single-precision%29) (DamageType :type Damage%20Type%20Object%20Reference) (InstigatedBy :type Controller%20Object%20Reference) (DamageCauser :type Actor%20Object%20Reference))
  (Default|RemoveHealthEvent (Variables|Default|GetAC_HealthSystem) Damage))

(fn ConstructionScript)