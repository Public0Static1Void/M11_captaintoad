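; BP_char_enemy is an AI enemy character that damages the player on contact and takes damage through a health system component.
; Capsule hits deal damage to BP_Character with a short cooldown; incoming damage removes health with knockback along the causer's forward vector, and death disables both.
; AI perception writes the seen player and position to the blackboard, and a Tick timer clears the target after a few seconds without perception updates.
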(event OnTargetPerceptionUpdated(AIPerception)
  (params (Actor :type Actor%20Object%20Reference) (Stimulus :type AI%20Stimulus%20Structure))
  (bind _returnvalue (AI|GetBlackboard 0))
  (bind _asbp_character (Utilities|Casting|CastToBP_Character Actor))
  (AI|Components|Blackboard|SetValueasObject _returnvalue (Utilities|Name|MakeLiteralName "Target") _asbp_character)
  (AI|Components|Blackboard|SetValueasVector _returnvalue (Utilities|Name|MakeLiteralName "targetPos") (Transformation|GetActorLocation _asbp_character))
  (Variables|Default|Setseen_target true)
  (Variables|Default|Setseen_timer 0.0))

(event Die(AC_HealthSystem)
  (Variables|Default|Setdie true)
  (Variables|Default|SetCanDamage false))

(event OnComponentHit(CapsuleComponent)
  (params (HitComponent :type Primitive%20Component%20Object%20Reference) (OtherActor :type Actor%20Object%20Reference) (OtherComp :type Primitive%20Component%20Object%20Reference) (NormalImpulse :type Vector :default "0, 0, 0") (Hit :type Hit%20Result%20Structure%20%28by%20ref%29))
  (if (Variables|Default|GetcanDamage)
    (Variables|Default|SetcanDamage false)
    (Utilities|Casting|CastToBP_Character OtherActor
      (:then
        (Game|Damage|ApplyDamage OtherActor 1.0 0 self))
      (:CastFailed
        _))
    (Utilities|FlowControl|Delay 0.75)
    (Variables|Default|SetcanDamage true)))

(event EventTick
  (params (DeltaSeconds :type Float%20%28single-precision%29))
  (if (Variables|Default|Getseen_target)
    (bind _output_get (Variables|Default|Setseen_timer (+ DeltaSeconds (Variables|Default|Getseen_timer))))
    (if (>= _output_get 3.0)
      (Variables|Default|Setseen_target false)
      (AI|Components|Blackboard|SetValueasObject (AI|GetBlackboard 0) (Utilities|Name|MakeLiteralName "Target") 0))))

(event Game|Damage|EventAnyDamage
  (params (Damage :type Float%20%28single-precision%29) (DamageType :type Damage%20Type%20Object%20Reference) (InstigatedBy :type Controller%20Object%20Reference) (DamageCauser :type Actor%20Object%20Reference))
  (if (not (Variables|Default|Getdie))
    (Default|RemoveHealthEvent (Variables|Default|GetAC_HealthSystem) 1.0 (* (Transformation|GetActorForwardVector DamageCauser) 300))))

(fn ConstructionScript)